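; BP_MasterEnemy is a master enemy Blueprint with a widget-based health bar and a status component.
; On BeginPlay it casts the health bar widget to WBP_HP_Bar_Enemy, stores the reference and refreshes it from the StatusComponent.
; Its Damage event only prints the damage amount and the attacking actor's name, without changing health or updating the bar.
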(event `self.ReceiveBeginPlay`
  ;[1 1 1] Event Begin Play - Refresh HealthBar
  (bind _output_get (set `self.HealthBarRef` (cast `/Game/Yiw/Enemies/WBP_HP_Bar_Enemy` (`WidgetComponent.GetUserWidgetObject` (`self.WidgetHealthBar`)) :!pure true)))
  (`/Game/Yiw/Enemies/WBP_HP_Bar_Enemy.RefreshHealthBar` _output_get (`self.StatusComponent`)))

(event `/Game/Yiw/Blueprints/I_Interactions.ReceiveDamage`
  (params (DamageAmount :type "Float (double-precision)") (AttackingActor :type "Actor Object Reference"))
  (`KismetSystemLibrary.PrintString` (`KismetStringLibrary.Conv_DoubleToString` DamageAmount))
  (`KismetSystemLibrary.PrintString` (`KismetSystemLibrary.GetDisplayName` AttackingActor)))

(fn `UserConstructionScript`)